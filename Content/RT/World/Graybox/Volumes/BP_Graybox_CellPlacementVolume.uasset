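; BP_Graybox_CellPlacementVolume is a graybox actor that shows the placement volume of a single hex cell prism.
; Its construction script adds two cell prism meshes for the origin cell, sized by HexSize and LayerHeight through CellVolumeTransform.
; One spans the full cell footprint, and the other is scaled in plane by SafeInsetFraction to mark an inset safe area.
; It has no active runtime logic.
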(fn `UserConstructionScript`
  (bind _returnvalue (`KismetMathLibrary.MakeVector` 0.0))
  (bind _returnvalue_2 (`RTHexMapActor.GetCellPrismMesh`))
  (bind _rtcellid (make `RTCellId` 0))
  (bind _hexsize (`self.HexSize`))
  (bind _layerheight (`self.LayerHeight`))
  (bind _returnvalue_3 (`AddComponent|NODE_AddStaticMeshComponent-2` :`RelativeTransform` (`RTHexLibrary.CellVolumeTransform` _rtcellid _returnvalue _hexsize _layerheight 1.0)))
  (`StaticMeshComponent.SetStaticMesh` _returnvalue_3 _returnvalue_2)
  (bind _returnvalue_4 (`AddComponent|NODE_AddStaticMeshComponent-3` :`RelativeTransform` (`RTHexLibrary.CellVolumeTransform` _rtcellid _returnvalue _hexsize _layerheight (`self.SafeInsetFraction`))))
  (`StaticMeshComponent.SetStaticMesh` _returnvalue_4 _returnvalue_2))